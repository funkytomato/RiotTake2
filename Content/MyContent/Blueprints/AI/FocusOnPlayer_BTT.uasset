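; Behavior Tree task that makes the AI focus on the player character and refreshes player-related Blackboard data.
; On execute it sets controller focus on player 0 and writes that character's location to the target location key.
; It then copies CanSeePlayer from the MasterAIController into the Blackboard and succeeds, failing only if the controller cast fails.
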(event `self.ReceiveExecuteAI`
  (params (OwnerController :type "AIController Object Reference") (ControlledPawn :type "Pawn Object Reference"))
  (bind _returnvalue (`GameplayStatics.GetPlayerCharacter` 0))
  (`AIController.K2_SetFocus` OwnerController _returnvalue)
  (`BTFunctionLibrary.SetBlackboardValueAsVector` (`self.BBTargetLocation`) (`Actor.K2_GetActorLocation` _returnvalue))
  (bind _asmaster_aicontroller (cast `/Game/MyContent/Blueprints/AI/MasterAIController` (`AIBlueprintHelperLibrary.GetAIController` ControlledPawn))
    (:`then`
      (`BTFunctionLibrary.SetBlackboardValueAsBool` (`self.BBCanSeePlayer`) (`/Game/MyContent/Blueprints/AI/MasterAIController.CanSeePlayer` _asmaster_aicontroller))
      (`self.FinishExecute` true))
    (:`CastFailed`
      (`self.FinishExecute` false))))