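; Zombie NPC Blueprint that handles melee attack montages and chase state through callable events.
; Attack skips if a montage is playing; crawling triggers both leg bites, while standing picks neck, left-swing or right-swing from AttackType.
; ProcessAttackType derives that type from the left/right attack flags.
; Capsule hit and sphere overlap events are empty, with the old proximity-attack logic left disconnected, so nothing here calls Attack.
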(event `NeckAttack`
  ;[1 1 1] Standing Attack
  (`|PlayMontage` (`self.Mesh`) "/Game/MyContent/Animations/Zombie/Standing/Attacking/AS_NAAT_Zombie_Attack_BH_Stand_Montage.AS_NAAT_Zombie_Attack_BH_Stand_Montage"))

(event `BiteLeftLeg`
  ;[1 1 1] Crawl Attack
  (if (`self.IsCrawling?`)
    (set `self.IsAttacking?` true)
    (set `self.IsLeftAttack?` true)
    (`|PlayMontage` (`self.Mesh`) "/Game/MyContent/Animations/Zombie/Crawl/AS_NAAT_Zombie_Attack_LH_Crawl_Montage.AS_NAAT_Zombie_Attack_LH_Crawl_Montage")))

(event `StartChase`
  ;[1 1 1] Chase
  (set `self.IsChasing?` true))

(event `StopChase`
  ;[1 1 1] Chase
  (set `self.IsChasing?` false))

(event `LeftSwingAttack`
  ;[1 1 1] Standing Attack
  (`|PlayMontage` (`self.Mesh`) "/Game/MyContent/Animations/Zombie/Standing/Attacking/AS_NAAT_Zombie_Attack_LH_Stand_Montage.AS_NAAT_Zombie_Attack_LH_Stand_Montage"))

(event `BiteRightLeg`
  ;[1 1 1] Crawl Attack
  (if (`self.IsCrawling?`)
    (set `self.IsAttacking?` true)
    (set `self.IsRightAttack?` true)
    (`|PlayMontage` (`self.Mesh`) "/Game/MyContent/Animations/Zombie/Crawl/AS_NAAT_Zombie_Attack_RH_Crawl_Montage.AS_NAAT_Zombie_Attack_RH_Crawl_Montage")))

(event `RightSwingAttack`
  ;[1 1 1] Standing Attack
  (`|PlayMontage` (`self.Mesh`) "/Game/MyContent/Animations/Zombie/Standing/Attacking/AS_NAAT_Zombie_Attack_RH_Stand_Montage.AS_NAAT_Zombie_Attack_RH_Stand_Montage"))

(event `Attack`
  (if (not (`AnimInstance.IsAnyMontagePlaying` (`SkeletalMeshComponent.GetAnimInstance` (`self.Mesh`))))
    ;[1 1 1] Attack
    (set `self.IsAttacking?` true)
    (`self.ProcessAttackType`)
    (if (`self.IsCrawling?`)
      (`self.BiteLeftLeg`)
      (`self.BiteRightLeg`)
      (else
        (switch `int` (`self.AttackType`)
          (:`0`
            (`self.NeckAttack`))
          (:`1`
            (`self.LeftSwingAttack`))
          (:`2`
            (`self.RightSwingAttack`)))))))

(event `StopAttack`
  ;[1 1 1] Attack
  (set `self.IsAttacking?` false))

(event `self.CapsuleComponent.OnComponentHit`
  (params (HitComponent :type "PrimitiveComponent Object Reference") (OtherActor :type "Actor Object Reference") (OtherComp :type "PrimitiveComponent Object Reference") (NormalImpulse :type "Vector Structure") (Hit :type "HitResult Structure (by ref)"))
  ;[1 1 1] Attack when Player close
)

(event `self.Sphere.OnComponentBeginOverlap`
  (params (OverlappedComponent :type "PrimitiveComponent Object Reference") (OtherActor :type "Actor Object Reference") (OtherComp :type "PrimitiveComponent Object Reference") (OtherBodyIndex :type Integer) (bFromSweep :type Boolean) (SweepResult :type "HitResult Structure (by ref)"))
  ;[1 1 1] Attack Influence
)

(event `self.Sphere.OnComponentEndOverlap`
  (params (OverlappedComponent :type "PrimitiveComponent Object Reference") (OtherActor :type "Actor Object Reference") (OtherComp :type "PrimitiveComponent Object Reference") (OtherBodyIndex :type Integer))
  ;[1 1 1] Attack Influence
)

(fn `ProcessAttackType`
  (if (and (`self.IsLeftAttack?`) (`self.IsRightAttack?`))
    (set `self.AttackType` 0)
    (elif (`self.IsLeftAttack?`)
      (set `self.AttackType` 1)
      (elif (`self.IsRightAttack?`)
        (set `self.AttackType` 2)))))

(fn `UserConstructionScript`
  (`parent.UserConstructionScript`))