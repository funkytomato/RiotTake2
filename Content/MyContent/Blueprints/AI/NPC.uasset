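; NPC character Blueprint that tracks health and energy, links itself to its NPC_WBP widget and reacts to damage.
; Capsule hits from weapons or projectiles apply point damage, and AnyDamage lowers clamped health, sets IsDead and plays a montage.
; The bound OnHit message plays a montage, briefly sets IsHit, and passes the montage's return value as damage.
; Health and energy message handlers are empty, and DecreaseEnergy sets HasEnergy inverted.
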(event `self.ReceiveBeginPlay`
  (add `self.UpdateHealthMsg` (delegate `UpdateHealthMsg_Event`))
  (add `self.UpdateEnergyMsg` (delegate `UpdateEnergyMsg_Event`))
  (add `self.OnHitMsg` (delegate `OnHitMsg_Event`))
  (bind _asnpc_wbp (cast `/Game/MyContent/Blueprints/UI/NPC_WBP` (`WidgetComponent.GetUserWidgetObject` (`self.Widget`))))
  (set `self.HealthWidget` _asnpc_wbp)
  (set `/Game/MyContent/Blueprints/UI/NPC_WBP.Owner` self _asnpc_wbp))

(event `UpdateHealthMsg_Event` :!signature `self.UpdateHealthMsg`
  (params (amount :type "Float (double-precision)")))

(event `UpdateEnergyMsg_Event` :!signature `self.UpdateEnergyMsg`
  (params (amount :type "Float (double-precision)")))

(event `OnHitMsg_Event` :!signature `self.OnHitMsg`
  (params (value :type "Float (double-precision)"))
  (`self.OnHit`))

(event `self.ReceiveAnyDamage`
  (params (Damage :type "Float (single-precision)") (DamageType :type "DamageType Object Reference") (InstigatedBy :type "Controller Object Reference") (DamageCauser :type "Actor Object Reference"))
  ;[1 1 1] Apply Damage and reduce Health, check if Dead
  (`self.DecreaseHealth` Damage))

(event `OnHit`
  (`KismetSystemLibrary.PrintString` "NPC OnHit")
  (set `self.IsHit?` true)
  (bind _returnvalue (`AnimInstance.Montage_Play` (`SkeletalMeshComponent.GetAnimInstance` (`self.Mesh`)) null 1.0 "MontageLength" 0.0 true))
  (`self.DecreaseHealth` _returnvalue)
  (`KismetSystemLibrary.Delay` 1.0)
  (set `self.IsHit?` false))

(event `self.CapsuleComponent.OnComponentHit`
  (params (HitComponent :type "PrimitiveComponent Object Reference") (OtherActor :type "Actor Object Reference") (OtherComp :type "PrimitiveComponent Object Reference") (NormalImpulse :type "Vector Structure") (Hit :type "HitResult Structure (by ref)"))
  ;[1 1 1] Apply Point Damage from Melee and Projectiles
  (bind _asweapon_master_bp (cast `/Game/MyContent/Blueprints/Weapons/WeaponMaster_BP` OtherActor)
    (:`then`
      (`GameplayStatics.ApplyPointDamage` self (`/Game/MyContent/Blueprints/Weapons/WeaponMaster_BP.DamageValue` _asweapon_master_bp) NormalImpulse Hit null _asweapon_master_bp))
    (:`CastFailed`
      (bind _asprojectile_master_bp (cast `/Game/MyContent/Blueprints/Weapons/Projectiles/ProjectileMaster_BP` OtherActor))
      (`GameplayStatics.ApplyPointDamage` self (`/Game/MyContent/Blueprints/Weapons/Projectiles/ProjectileMaster_BP.DamageAmount` _asprojectile_master_bp) NormalImpulse Hit))))

(fn `DecreaseEnergy`
  (params (Amount :type "Float (double-precision)"))
  (bind _output_get (set `self.Energy` (`KismetMathLibrary.FClamp` (- (`self.Energy`) Amount) 0.0 (`self.MaxEnergy`))))
  (set `self.HasEnergy?` (not (> _output_get 0.0))))

(fn `DecreaseHealth`
  (params (Amount :type "Float (double-precision)"))
  (bind _output_get (set `self.Health` (`KismetMathLibrary.FClamp` (- (`self.Health`) Amount) 0.0 (`self.MaxHealth`))))
  (set `self.IsDead?` (<= _output_get 0.0))
  (`AnimInstance.Montage_Play` (`SkeletalMeshComponent.GetAnimInstance` (`self.Mesh`)) null 1.0 "MontageLength" 0.0 true))

(fn `IncreaseEnergy`
  (params (Amount :type "Float (double-precision)"))
  (bind _output_get (set `self.Energy` (`KismetMathLibrary.FClamp` (+ (`self.Energy`) Amount) 0.0 (`self.MaxEnergy`))))
  (set `self.HasEnergy?` (> _output_get 0.0)))

(fn `IncreaseHealth`
  (params (Amount :type "Float (double-precision)"))
  (set `self.Health` (`KismetMathLibrary.FClamp` (+ (`self.Health`) Amount) 0.0 (`self.MaxHealth`))))

(fn `UserConstructionScript`)