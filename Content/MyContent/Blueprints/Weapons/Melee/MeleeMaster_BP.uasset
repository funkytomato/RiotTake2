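; MeleeMaster_BP is a melee weapon Blueprint, apparently a base for melee weapons, that handles attacking and dropping when broken.
; Attack prints a debug message, then calls UseItem, or DropWeapon if IsBroken is set.
; DropWeapon detaches the owner's EquippedWeapon and destroys this actor after a short delay.
; StopAttack is empty, and the strike montage logic is disconnected, so it never runs.
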(event `StopAttack`)

(event `Attack`
  (`KismetSystemLibrary.PrintString` "Melee Attacking")
  (if (not (`self.IsBroken?`))
    (`self.UseItem`)
    (else
      (`self.DropWeapon`))))

(event `DropWeapon`
  (`self.K2_DetachFromActor` (`/Game/MyContent/Blueprints/Player/MyPlayerCharacter.EquippedWeapon` (`self.WeaponOwner`)) "KeepRelative" "KeepRelative" "KeepRelative")
  (`KismetSystemLibrary.Delay` 2.0)
  (`self.K2_DestroyActor`))

(fn `UserConstructionScript`
  (`parent.UserConstructionScript`))