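; Master weapon Blueprint that tracks durability and a broken state.
; The construction script caches its owner by casting the parent actor to PlayerCharacter, which relies on the weapon being a child actor of the player.
; UseItem passes the weapon's DamageValue to ReduceDurability as the wear amount.
; ReduceDurability clamps durability to a fixed range and sets IsBroken from whether it has run out.
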(fn `ReduceDurability`
  (params (amount :type "Float (double-precision)"))
  (bind _output_get (set `self.Durability` (`KismetMathLibrary.FClamp` (- (`self.Durability`) amount) 0.0 100.0)))
  (set `self.IsBroken?` (<= _output_get 0.0)))

(fn `UseItem`
  (`self.ReduceDurability` (`self.DamageValue`)))

(fn `UserConstructionScript`
  (bind _asplayer_character (cast `/Game/MyContent/Blueprints/Player/PlayerCharacter` (`self.GetParentActor`)))
  (set `self.WeaponOwner` _asplayer_character))