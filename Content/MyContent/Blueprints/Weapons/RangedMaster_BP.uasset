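; Base ranged weapon Blueprint, attached as a child actor of the player character, that handles automatic fire, ammo and reloading.
; StartShooting fires at once and loops FireProjectile on a FireRate timer until StopShooting clears it.
; Each shot with ammo left spawns a ProjectileMaster_BP at the barrel point along the character mesh's rotation, plays a montage and decrements ammo.
; Reload refills the clip from the reserve, taking whatever remains when short.
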(event `self.ReceiveBeginPlay`
  (`parent.ReceiveBeginPlay`)
  (bind _asplayer_character (cast `/Game/MyContent/Blueprints/Player/PlayerCharacter` (`self.GetParentActor`)))
  (bind _output_get (set `self.PlayerCharacter` _asplayer_character))
  (set `self.AnimInstance` (`SkeletalMeshComponent.GetAnimInstance` (`Character.Mesh` _output_get))))

(event `StartShooting`
  (set `self.IsFiring` true)
  (`self.FireProjectile`)
  (bind _returnvalue (`KismetSystemLibrary.K2_SetTimer` null "FireProjectile" (`self.FireRate`) true))
  (set `self.FireProjectileTimer` _returnvalue))

(event `StopShooting`
  (set `self.IsFiring` false)
  (`KismetSystemLibrary.K2_ClearAndInvalidateTimerHandle` (`self.FireProjectileTimer`)))

(fn `FireProjectile`
  (if (> (`self.AmmoCount`) 0)
    (`|SpawnActorFromClass` "/Game/MyContent/Blueprints/Weapons/ProjectileMaster_BP.ProjectileMaster_BP_C" (`KismetMathLibrary.MakeTransform` (`SceneComponent.K2_GetComponentLocation` (`self.BarrelRefPoint`)) (`SceneComponent.K2_GetComponentRotation` (`Character.Mesh` (`self.PlayerCharacter`)))) "AlwaysSpawn" "OverrideRootScale" null null)
    (`AnimInstance.Montage_Play` (`self.AnimInstance`) null 1.0 "MontageLength" 0.0 true)
    (`/Engine/EditorBlueprintResources/StandardMacros.DecrementInt` (`self.AmmoCount`))))

(fn `Reload`
  (set `self.BulletDifference` (- (`self.ClipSize`) (`self.AmmoCount`)))
  (if (>= (`self.AmmoMax`) (`self.BulletDifference`))
    (set `self.AmmoCount` (`self.ClipSize`))
    (set `self.AmmoMax` (- (`self.AmmoMax`) (`self.BulletDifference`)))
    (else
      (set `self.AmmoCount` (+ (`self.AmmoCount`) (`self.AmmoMax`)))
      (set `self.AmmoMax` 0))))

(fn `UserConstructionScript`
  (`parent.UserConstructionScript`))