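; Base explodable actor that accumulates damage from projectile contact, general damage events and an IncreaseDamage message.
; Capsule hit and overlap events apply damage using a projectile's DamageAmount, and AnyDamage feeds it into IncreaseDamage.
; IncreaseDamage adds to a clamped Damage value, flags IsDestroyed only at zero or below, and calls Explode on every call.
; Explode activates the Niagara effect and enables ProjectileMovement simulation.
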(event `self.ReceiveBeginPlay`
  (add `self.IncreaseDamageMsg` (delegate `IncreaseDamageMsg_Event`)))

(event `IncreaseDamageMsg_Event` :!signature `self.IncreaseDamageMsg`
  (params (amount :type "Float (double-precision)"))
  (`self.IncreaseDamage` amount))

(event `Explode`
  (bind _niagara (`self.Niagara`))
  (`ActorComponent.SetAutoActivate` _niagara true)
  (`ActorComponent.SetActive` _niagara true true)
  (set `ProjectileMovementComponent.bSimulationEnabled` true (`self.ProjectileMovement`)))

(event `self.Capsule.OnComponentHit`
  (params (HitComponent :type "PrimitiveComponent Object Reference") (OtherActor :type "Actor Object Reference") (OtherComp :type "PrimitiveComponent Object Reference") (NormalImpulse :type "Vector Structure") (Hit :type "HitResult Structure (by ref)"))
  (cast `/Game/MyContent/Blueprints/Player/MyPlayerCharacter` OtherActor
    (:`then`
      _)
    (:`CastFailed`
      (bind _asprojectile_master_bp (cast `/Game/MyContent/Blueprints/Weapons/Projectiles/ProjectileMaster_BP` OtherActor))))
  (`GameplayStatics.ApplyDamage` null (`/Game/MyContent/Blueprints/Weapons/Projectiles/ProjectileMaster_BP.DamageAmount` _asprojectile_master_bp)))

(event `self.Capsule.OnComponentBeginOverlap`
  (params (OverlappedComponent :type "PrimitiveComponent Object Reference") (OtherActor :type "Actor Object Reference") (OtherComp :type "PrimitiveComponent Object Reference") (OtherBodyIndex :type Integer) (bFromSweep :type Boolean) (SweepResult :type "HitResult Structure (by ref)"))
  (bind _asprojectile_master_bp (cast `/Game/MyContent/Blueprints/Weapons/Projectiles/ProjectileMaster_BP` OtherActor))
  (`GameplayStatics.ApplyDamage` self (`/Game/MyContent/Blueprints/Weapons/Projectiles/ProjectileMaster_BP.DamageAmount` _asprojectile_master_bp) null _asprojectile_master_bp))

(event `self.ReceiveAnyDamage`
  (params (Damage :type "Float (single-precision)") (DamageType :type "DamageType Object Reference") (InstigatedBy :type "Controller Object Reference") (DamageCauser :type "Actor Object Reference"))
  (`self.IncreaseDamage` Damage))

(fn `IncreaseDamage`
  (params (amount :type "Float (double-precision)"))
  (bind _output_get (set `self.Damage` (`KismetMathLibrary.FClamp` (+ (`self.Damage`) amount) 0.0 100.0)))
  (set `self.IsDestroyed?` (<= _output_get 0.0))
  (`self.Explode`))

(fn `UserConstructionScript`)